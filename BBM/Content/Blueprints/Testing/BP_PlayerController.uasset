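; Test player controller that moves the first player's pawn across the X/Y plane and reports its position.
; The Vertical and Horizontal axis inputs add their raw values to the pawn's X and Y location through SetActorLocation, without delta-time scaling.
; Pressing Space prints the pawn's rounded X, Y and Z coordinates as a debug string.
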(event EventBeginPlay)

(event EventTick
  (params (DeltaSeconds :type Float%20%28single-precision%29)))

(event Input|ActionEvents|InputActionSpace
  (params (Key :type Key%20Structure :default "None"))
  (bind _returnvalue (Game|Player|GetPlayerPawn 0))
  (bind _returnvalue_2 (Transformation|GetActorLocation _returnvalue))
  (:Pressed
    (Development|PrintString (Utilities|String|Append "X= " (Utilities|String|ToString(Integer) (Math|Float|Round (.x _returnvalue_2))) "Y= " (Utilities|String|ToString(Integer) (Math|Float|Round (.y _returnvalue_2))) "Z= " (Utilities|String|ToString(Integer) (Math|Float|Round (.z _returnvalue_2)))))))

(event Input|AxisEvents|InputAxisVertical_Axis
  (params (AxisValue :type Float%20%28single-precision%29))
  (bind _returnvalue (Game|Player|GetPlayerPawn 0))
  (bind _returnvalue_2 (Transformation|GetActorLocation _returnvalue))
  (Transformation|SetActorLocation _returnvalue (Math|Vector|MakeVector (+ (.x _returnvalue_2) AxisValue) (.y _returnvalue_2) (.z _returnvalue_2)) false false))

(event Input|AxisEvents|InputAxisHorizontal_Axis
  (params (AxisValue :type Float%20%28single-precision%29))
  (bind _returnvalue (Game|Player|GetPlayerPawn 0))
  (bind _returnvalue_2 (Transformation|GetActorLocation _returnvalue))
  (Transformation|SetActorLocation _returnvalue (Math|Vector|MakeVector (.x _returnvalue_2) (+ (.y _returnvalue_2) AxisValue) (.z _returnvalue_2)) false false))

(fn ConstructionScript)